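; Test-task Blueprint that moves a sphere continuously along a spline while it leaves a particle trail.
; Each Tick sets the sphere's relative location from the spline's local position at the current time, then advances that time by delta seconds, wrapped within the spline's duration so the motion loops.
; BeginPlay starts the particle trail between two named sockets, with width measured from the centre.
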(event `self.ReceiveBeginPlay`
  (`ParticleSystemComponent.BeginTrails` (`self.P_Trail`) "Trail1" "Trail2" "ETrailWidthMode_FromCentre" 3.0))

(event `self.ReceiveTick`
  (params (DeltaSeconds :type "Float (single-precision)"))
  (`|ExecutionSequence`
    (:`then_0`
      (`SceneComponent.K2_SetRelativeLocation` (`self.TTSphere`) (`SplineComponent.GetLocationAtTime` (`self.Spline`) (`self.SplineTime`) "Local" false) false false))
    (:`then_1`
      (set `self.SplineTime` (`KismetMathLibrary.FWrap` (+ DeltaSeconds (`self.SplineTime`)) 0.0 (`SplineComponent.Duration` (`self.Spline`)))))))

(fn `UserConstructionScript`)